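; BP_SpiderCannon is a spider turret that turns to face the player and periodically fires projectiles.
; Tick rotates the capsule toward player pawn 0.
; A looping timer spawns BP_SpiderProjectile from the mesh's MouthSocket with the actor's rotation and plays the firewall animation.
; A slower looping "chase" timer only plays the charge animation, with no movement logic.
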(event `self.ReceiveBeginPlay`
  (`KismetSystemLibrary.K2_SetTimerDelegate` (delegate `OnTimerFireElapsed`) 3.0 true)
  (`KismetSystemLibrary.K2_SetTimerDelegate` (delegate `OnChaseTimerElapsed`) 10.0 true))

(event `OnTimerFireElapsed`
  (`|SpawnActorFromClass` "/Game/Rogue/Blueprints/ForTesting/BP_SpiderProjectile.BP_SpiderProjectile_C" (`KismetMathLibrary.MakeTransform` (`SceneComponent.GetSocketLocation` (`self.Mesh`) "MouthSocket") (`self.K2_GetActorRotation`)) "Undefined" "OverrideRootScale" null null)
  (`SkeletalMeshComponent.PlayAnimation` (`self.Mesh`) "/Game/ExampleContent/Enemy_Great_Spider/Animation/AM_Spider_Firewall.AM_Spider_Firewall" false))

(event `OnChaseTimerElapsed`
  (`SkeletalMeshComponent.PlayAnimation` (`self.Mesh`) "/Game/ExampleContent/Enemy_Great_Spider/Animation/AM_Spider_Charge.AM_Spider_Charge" false))

(event `self.ReceiveTick`
  (params (DeltaSeconds :type "Float (single-precision)"))
  (`SceneComponent.K2_SetWorldRotation` (`self.CapsuleComponent`) (`KismetMathLibrary.FindLookAtRotation` (`self.K2_GetActorLocation`) (`self.K2_GetActorLocation` (`GameplayStatics.GetPlayerPawn` 0))) false false))

(fn `UserConstructionScript`)