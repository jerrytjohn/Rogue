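; BP_Door is a double door that swings open when its ToggleDoor event fires.
; Timelines drive the relative yaw of the right and left door meshes, with the left timeline played from the right one's update.
; IsClosed clears when the left swing finishes.
; A mirrored closing sequence that sets IsClosed exists but is disconnected, so ToggleDoor only opens the door.
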(event `ToggleDoor`
  (bind (_direction _door_yaw) (`Timeline|Right Door Yaw Swing Open`)
    (:`Update`
      (`SceneComponent.K2_SetRelativeRotation` (`self.SM_DoorRight`) (`KismetMathLibrary.MakeRotator` 0.0 0.0 _door_yaw) false false)
      (bind (_direction_2 _door_yaw_2) (`Timeline|Left Door Yaw Swing Open`)
        (:`Update`
          (`SceneComponent.K2_SetRelativeRotation` (`self.SM_DoorLeft`) (`KismetMathLibrary.MakeRotator` 0.0 0.0 _door_yaw_2) false false))
        (:`Finished`
          (set `self.bIsClosed` false))))))

(fn `UserConstructionScript`)